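; Custom PCG Blueprint node that resizes point bounds into column-like boxes whose height follows point density.
; ExecuteWithContext converts the first input's spatial data to points, runs the point loop and returns the result as a data collection.
; PointLoopBody sets a fixed XY footprint and scales the upper Z bound by density, but returns false for every point, which normally discards it from the output.
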(fn ExecutewithContext
  (params (InContext :type PCG%20Context%20Structure%20%28by%20ref%29) (Input :type PCG%20Data%20Collection%20Structure%20%28by%20ref%29))
  (bind _returnvalue (Class|PCGDataFunctionLibrary|GetInputs Input))
  (bind _aspcg空间数据 (Utilities|Casting|CastToPCGSpatialData (.Data (Utilities|Struct|BreakPCGTaggedData (Utilities|Array|Get(acopy) _returnvalue))))
    (:then
      (bind _outdata (PCG|FlowControl|PointLoop InContext (SpatialData|ToPointDatawithContext _aspcg空间数据 InContext) 0))
      (return (Utilities|Struct|MakePCGDataCollection (Utilities|Array|MakeArray (Utilities|Struct|MakePCGTaggedData _outdata 0 "None")))))
    (:CastFailed
      (return ""))))

(fn PointLoopBody
  (params (InContext :type PCG%20Context%20Structure%20%28by%20ref%29) (InData :type PCG%20Point%20Data%20Object%20Reference) (InPoint :type PCG%20Point%20Structure%20%28by%20ref%29) (OutMetadata :type PCG%20Metadata%20Object%20Reference) (Iteration :type Integer64))
  (bind _structout (Utilities|Struct|SetmembersinPCGPoint InPoint "-50.000000,-50.000000,-1.000000" (Math|Vector|MakeVector 5e+01 5e+01 (* (.Density (Utilities|Struct|BreakPCGPoint InPoint)) 1e+03))))
  (return _structout false))