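; Base Blueprint for building pieces that shows a placement preview and turns into the placed object.
; On BeginPlay it caches the mesh's original materials, then applies the invalid-placement preview material.
; SetMaterialPreview swaps every material slot between the valid and error preview material instances based on placement validity.
; PlaceObject, only when placement is valid, restores the cached materials and clears the preview flag.
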(event Custom|PlaceObject
  (if (Variables|Default|GetIsVailedPlacement)
    (for (_array_element _array_index) (Variables|Default|GetMaterials)
      (Rendering|Material|SetMaterial (Variables|Default|GetMesh) _array_index _array_element))
    (Variables|Default|SetIsPreview false)))

(event EventBeginPlay
  (Variables|Default|SetMaterials (Rendering|Material|GetMaterials (Variables|Default|GetMesh)))
  (CallFunction|SetMaterialPreview false))

(event Collision|EventActorBeginOverlap
  (params (OtherActor :type Actor%20Object%20Reference)))

(event EventTick
  (params (DeltaSeconds :type Float%20%28single-precision%29)))

(fn ConstructionScript)

(fn SetMaterialPreview
  (params (IsVailedPlacement :type Boolean))
  (Variables|Default|SetPreviewMaterial (select IsVailedPlacement "/Game/PrimaryData/M_BuildPrevirew_Inst.M_BuildPrevirew_Inst" "/Game/PrimaryData/M_BuildPrevirew_Inst_error.M_BuildPrevirew_Inst_error"))
  (for _index (range 0 (Utilities|Array|LastIndex (Variables|Default|GetMaterials)))
    (Rendering|Material|SetMaterial (Variables|Default|GetMesh) _index (Variables|Default|GetPreviewMaterial))))